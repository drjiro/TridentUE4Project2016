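; GameMode Blueprint that holds inversion flags for camera and X/Y aim controls, with its logic left unfinished.
; The TurnCameraLeft press checks the camera inversion flag but performs no action.
; Disconnected nodes would copy the flags from checkboxes in the main and pause menu widgets, but they never run.
; BeginPlay, Tick and the construction script are empty.
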(event EventBeginPlay)

(event EventTick
  (params (DeltaSeconds :type Float%20%28single-precision%29)))

(event Input|ActionEvents|InputActionTurnCameraLeft
  (params (Key :type Key%20Structure :default "AnyKey"))
  (:Pressed
    (if (Variables|Default|GetIsInvertedCamera)
      _)))

(fn ConstructionScript)