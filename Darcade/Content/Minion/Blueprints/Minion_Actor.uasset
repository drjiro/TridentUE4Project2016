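; Flocking enemy minion that seeks a target, attacks the player and dies to weapon hits.
; Each tick steers toward Target plus boids forces from nearby minions, then turns and steps a fixed distance forward; Cohesion's loop input is unwired.
; Range overlaps set a chase flag, unread here, or pause movement for a timed attack.
; Belly and back each require a different weapon ID to kill, updating the spawner and enabling physics before delayed destruction.
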(event OnComponentBeginOverlap(SearchEnemyRange)
  (params (OverlappedComponent :type Primitive%20Component%20Object%20Reference) (OtherActor :type Actor%20Object%20Reference) (OtherComp :type Primitive%20Component%20Object%20Reference) (OtherBodyIndex :type Integer) (bFromSweep :type Boolean) (SweepResult :type Hit%20Result%20Structure%20%28by%20ref%29))
  ;[1 1 1] Discover the player
  (Utilities|Casting|CastToPrideCharacter OtherActor)
  (if (not (Variables|OpenParam|GetIsKilled))
    (Variables|OpenParam|SetIsChasing true)))

(event OnComponentBeginOverlap(AttackRange)
  (params (OverlappedComponent :type Primitive%20Component%20Object%20Reference) (OtherActor :type Actor%20Object%20Reference) (OtherComp :type Primitive%20Component%20Object%20Reference) (OtherBodyIndex :type Integer) (bFromSweep :type Boolean) (SweepResult :type Hit%20Result%20Structure%20%28by%20ref%29))
  ;[1 1 1] Attack Preparation
  (Utilities|Casting|CastToPrideCharacter OtherActor)
  (if (not (Variables|OpenParam|GetIsKilled))
    (if (not (Variables|Default|GetIsAttackPreparation))
      (Variables|Default|SetIsAttackPreparation true)
      (Components|Animation|PlayAnimation (Variables|Default|GetSkeletalMesh) "/Game/Minion/Animations/Minion_Attack_LegSucker_Anim.Minion_Attack_LegSucker_Anim" false)
      (Utilities|FlowControl|Delay 3.0)
      (Variables|Default|SetIsAttackPreparation false))))

(event OnComponentEndOverlap(SearchEnemyRange)
  (params (OverlappedComponent :type Primitive%20Component%20Object%20Reference) (OtherActor :type Actor%20Object%20Reference) (OtherComp :type Primitive%20Component%20Object%20Reference) (OtherBodyIndex :type Integer))
  ;[1 1 1] Missing the player
  (Utilities|Casting|CastToPrideCharacter OtherActor)
  (if (not (Variables|OpenParam|GetIsKilled))
    (Variables|OpenParam|SetIsChasing false)))

(event OnComponentBeginOverlap(BackCollision)
  (params (OverlappedComponent :type Primitive%20Component%20Object%20Reference) (OtherActor :type Actor%20Object%20Reference) (OtherComp :type Primitive%20Component%20Object%20Reference) (OtherBodyIndex :type Integer) (bFromSweep :type Boolean) (SweepResult :type Hit%20Result%20Structure%20%28by%20ref%29))
  (bind _minionspawnerrefarence (Variables|Default|GetMinionSpawnerRefarence))
  (bind _minions (Variables|/Game/Minion/Blueprints/MinionSpawner.MinionSpawner_C|GetMinions _minionspawnerrefarence))
  ;[1 1 1] Back Hit Flow
  (if (not (Variables|OpenParam|GetIsKilled))
    (if (Components|ComponentHasTag OtherComp "WeaponCollision")
      (bind _aspride_character (Utilities|Casting|CastToPrideCharacter OtherActor))
      (if (Utilities|Enum|Equal(Enum) (Variables|/Game/PlayerCharacter/Blueprints/PrideCharacter.PrideCharacter_C|GetWeaponID _aspride_character) "NewEnumerator1")
        (for (_array_element _array_index) _minions
          (if (== _array_element self)
            (Components|Animation|PlayAnimation (Variables|Default|GetSkeletalMesh) "/Game/Minion/Animations/Minion_Death_Anim.Minion_Death_Anim" false)
            (Variables|OpenParam|SetIsKilled true)
            (Variables|Default|SetIsAttackPreparation false)
            (Utilities|Array|RemoveIndex _minions _array_index)
            (Math|Integer|IncrementInt (Variables|/Game/Minion/Blueprints/MinionSpawner.MinionSpawner_C|GetKilledMinion (Variables|Default|GetMinionSpawnerRefarence))
              (:%20%20
                (Physics|SetSimulatePhysics (Variables|Default|GetSkeletalMesh) true) ; off simulate
                (Utilities|FlowControl|Delay 15.0)
                (Actor|DestroyActor)))))))))

(event OnComponentBeginOverlap(BellyCollision)
  (params (OverlappedComponent :type Primitive%20Component%20Object%20Reference) (OtherActor :type Actor%20Object%20Reference) (OtherComp :type Primitive%20Component%20Object%20Reference) (OtherBodyIndex :type Integer) (bFromSweep :type Boolean) (SweepResult :type Hit%20Result%20Structure%20%28by%20ref%29))
  (bind _minionspawnerrefarence (Variables|Default|GetMinionSpawnerRefarence))
  (bind _minions (Variables|/Game/Minion/Blueprints/MinionSpawner.MinionSpawner_C|GetMinions _minionspawnerrefarence))
  ;[1 1 1] Belly Hit Flow
  (if (not (Variables|OpenParam|GetIsKilled))
    (if (Components|ComponentHasTag OtherComp "WeaponCollision")
      (bind _aspride_character (Utilities|Casting|CastToPrideCharacter OtherActor))
      (if (Utilities|Enum|Equal(Enum) (Variables|/Game/PlayerCharacter/Blueprints/PrideCharacter.PrideCharacter_C|GetWeaponID _aspride_character) "NewEnumerator0")
        (for (_array_element _array_index) _minions
          (if (== _array_element self)
            (Components|Animation|PlayAnimation (Variables|Default|GetSkeletalMesh) "/Game/Minion/Animations/Minion_Death_Anim.Minion_Death_Anim" false)
            (Variables|OpenParam|SetIsKilled true)
            (Variables|Default|SetIsAttackPreparation false)
            (Utilities|Array|RemoveIndex _minions _array_index)
            (Math|Integer|IncrementInt (Variables|/Game/Minion/Blueprints/MinionSpawner.MinionSpawner_C|GetKilledMinion (Variables|Default|GetMinionSpawnerRefarence))
              (:%20%20
                (Physics|SetSimulatePhysics (Variables|Default|GetSkeletalMesh) true) ; off simulate
                (Utilities|FlowControl|Delay 15.0)
                (Actor|DestroyActor)))))))))

(event EventBeginPlay)

(event Collision|EventActorBeginOverlap
  (params (OtherActor :type Actor%20Object%20Reference)))

(event EventTick
  (params (DeltaSeconds :type Float%20%28single-precision%29))
  ;[1 1 1] Flocking AI
  (Variables|Default|SetDeltaTime DeltaSeconds)
  (bind _outactors (Class|KismetSystemLibrary|SphereOverlapActorsNEW (Transformation|GetActorLocation) (Variables|/Script/Engine.SphereComponent|GetSphereRadius (Variables|Default|GetSearchEnemyRange)) (Utilities|Array|MakeArray "ObjectTypeQuery2") "Minion_Actor_C" (Utilities|Array|MakeArray self)))
  (CallFunction|Flock _outactors)
  (Variables|Default|SetVelocity (* (Math|Vector|Normalize (- (Transformation|GetWorldLocation (Variables|Default|GetTarget)) (Transformation|GetActorLocation))) (Variables|OpenParam|GetToTargetWeight)))
  (if (not (Variables|OpenParam|GetIsKilled))
    (if (not (Variables|Default|GetIsAttackPreparation))
      (CallFunction|Update))))

(fn ConstructionScript)

(fn Flock
  (params (Minions :type Array%20of%20Actor%20Object%20References))
  (bind _return (CallFunction|Separate Minions))
  (LocalVariables|SetSep _return)
  (bind _return_2 (CallFunction|Align Minions))
  (LocalVariables|SetAli _return_2)
  (bind _return_3 (CallFunction|Cohesion Minions))
  (LocalVariables|SetCoh _return_3)
  (CallFunction|ApplyForce (* (LocalVariables|GetSep) (Variables|OpenParam|GetSepWeight)))
  (CallFunction|ApplyForce (* (LocalVariables|GetAli) (Variables|OpenParam|GetAliWeight)))
  (CallFunction|ApplyForce (* (LocalVariables|GetCoh) (Variables|OpenParam|GetCohWeight))))

(fn Separate
  (params (minions :type Array%20of%20Actor%20Object%20References))
  (for _array_element minions
    (LocalVariables|SetOther _array_element)
    (if (and (> (Math|Vector|VectorLength (- (Transformation|GetActorLocation) (Transformation|GetActorLocation _array_element))) 0.0) true)
      (LocalVariables|SetSteer (+ (LocalVariables|GetSteer) (/ (Math|Vector|Normalize (- (Transformation|GetActorLocation) (Transformation|GetActorLocation (LocalVariables|GetOther)))) (Math|Vector|VectorLength (- (Transformation|GetActorLocation) (Transformation|GetActorLocation (LocalVariables|GetOther)))))))
      (Math|Integer|IncrementInt (LocalVariables|GetCount))))
  (if (> (LocalVariables|GetCount) 0)
    (bind _output_get (LocalVariables|SetSteer (/ (LocalVariables|GetSteer) (Math|Conversions|ToFloat(Integer) (LocalVariables|GetCount)))))
    (if (> (Math|Vector|VectorLength _output_get) 0.0)
      (return (Math|Vector|ClampVectorSize (- (Math|Vector|Normalize (LocalVariables|GetSteer)) (Variables|Default|GetVelocity)) 0.0 (Variables|OpenParam|GetMaxForce)))
      (else
        _)))
  (return "0, 0, 0"))

(fn Align
  (params (minions :type Array%20of%20Actor%20Object%20References))
  (for _array_element minions
    (if (and (> (Math|Vector|VectorLength (- (Transformation|GetActorLocation) (Transformation|GetActorLocation _array_element))) 0.0) true)
      (LocalVariables|SetSum (+ (LocalVariables|GetSum) (Transformation|GetVelocity _array_element)))
      (Math|Integer|IncrementInt (LocalVariables|GetCount))))
  (if (> (LocalVariables|GetCount) 0)
    (bind _output_get (LocalVariables|SetSum (/ (LocalVariables|GetSum) (Math|Conversions|ToFloat(Integer) (LocalVariables|GetCount)))))
    (return (Math|Vector|ClampVectorSize (- (* (Math|Vector|Normalize _output_get) (Variables|OpenParam|GetMaxSpeed)) (Variables|Default|GetVelocity)) 0.0 (Variables|OpenParam|GetMaxForce)))
    (else
      (return "0, 0, 0"))))

(fn Cohesion
  (params (minions :type Array%20of%20Actor%20Object%20References))
  (for _array_element 0
    (if (not (> (Math|Vector|VectorLength (- (Transformation|GetActorLocation) (Transformation|GetActorLocation _array_element))) 0.0))
      (LocalVariables|SetSum (- (LocalVariables|GetSum) (Transformation|GetActorLocation _array_element)))
      (Math|Integer|IncrementInt (LocalVariables|GetCount))))
  (if (> (LocalVariables|GetCount) 0)
    (bind _output_get (LocalVariables|SetSum (/ (LocalVariables|GetSum) (Math|Conversions|ToFloat(Integer) (LocalVariables|GetCount)))))
    (bind _return (CallFunction|Seek _output_get))
    (return _return)
    (else
      (return "0, 0, 0"))))

(fn Seek
  (params (target :type Vector))
  (return (Math|Vector|ClampVectorSize (- (* (Math|Vector|Normalize (- target (Transformation|GetActorLocation))) (Variables|OpenParam|GetMaxSpeed)) (Variables|Default|GetVelocity)) 0.0 (Variables|OpenParam|GetMaxForce))))

(fn ApplyForce
  (params (force :type Vector))
  (Variables|Default|SetAcceleration (+ (Variables|Default|GetAcceleration) force)))

(fn Update
  (bind _returnvalue (Transformation|GetActorLocation))
  (bind _output_get (Variables|Default|SetVelocity (+ (Variables|Default|GetVelocity) (Variables|Default|GetAcceleration))))
  (Variables|Default|SetVelocity (Math|Vector|ClampVectorSize _output_get 0.0 (Variables|OpenParam|GetMaxSpeed)))
  (Transformation|SetActorRotation (Math|Interpolation|RInterpTo (Transformation|GetActorRotation) (Math|Rotator|FindLookatRotation _returnvalue (+ _returnvalue (Variables|Default|GetVelocity))) (Variables|Default|GetDeltaTime) (Variables|OpenParam|GetMaxTurnRate)))
  (Transformation|AddActorLocalOffset "10.000000, 0, 0" false false)
  (Variables|Default|SetAcceleration (* (Variables|Default|GetAcceleration) 0.0)))