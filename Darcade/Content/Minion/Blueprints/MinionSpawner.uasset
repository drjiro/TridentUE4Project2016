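; MinionSpawner spawns a flock of Minion_Actors in a box around BossPoint and steers them between following the boss and chasing the player.
; All minions share the MinionsTarget component and receive initial flocking parameters at spawn.
; Tick updates BossPoint from the enemy reference, then moves the target, after a Delay, near the player if any minion is chasing, otherwise near the boss.
; It also copies live WID_Flocking values, except turn rate, onto living minions.
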(event EventBeginPlay
  ;[1 1 1] MinionSpawner - spawn minion
  (Rendering|SetVisibility (Variables|Default|GetMinionsTarget) false false)
  (bind _foundwidgets (Widget|GetAllWidgetsOfClass "/Game/Minion/Blueprints/WID_Flocking.WID_Flocking_C" true))
  (Variables|Default|SetWID_Flocking (Utilities|Array|Get(acopy) _foundwidgets))
  (for _index (range 0 (Variables|Default|GetNumSpawnMinion))
    (bind _returnvalue (Game|SpawnActorfromClass "/Game/Minion/Blueprints/Minion_Actor.Minion_Actor_C" (Math|Transform|MakeTransform (Math|Random|RandomPointinBoundingBox (Variables|Default|GetBossPoint) (Variables|Default|GetSpawnBoxSize)) "0, 0, 0" (Variables|Default|GetMinionScale)) "Undefined" 0 0))
    (Utilities|Array|AddUnique (Variables|Default|GetMinions) _returnvalue)
    (Variables|/Game/Minion/Blueprints/Minion_Actor.Minion_Actor_C|SetTarget _returnvalue (Variables|Default|GetMinionsTarget))
    (CallFunction|SetMinionParameters _returnvalue (Variables|Default|GetMaxForce) (Variables|Default|GetMaxSpeed) (Variables|Default|GetSepWeight) (Variables|Default|GetAliWeight) (Variables|Default|GetCohWeight) (Variables|Default|GetToTargetWeight) (Variables|Default|GetMaxTurnRate)))
  (Transformation|SetWorldLocation (Variables|Default|GetMinionsTarget) (Variables|Default|GetBossPoint) false false))

(event EventTick
  (params (DeltaSeconds :type Float%20%28single-precision%29))
  (bind _returnvalue (Game|GetPlayerCharacter 0))
  (bind _enemyrefarence (Variables|Default|GetEnemyRefarence))
  (bind _returnvalue_2 (Transformation|GetActorLocation _returnvalue))
  (bind _enemypos (Variables|/Game/AI/AI_Enemy.AI_Enemy_C|GetEnemyPos _enemyrefarence))
  (bind (_x _y) (Math|Vector|BreakVector _enemypos))
  (bind (_x_2 _y_2) (Math|Vector|BreakVector _returnvalue_2))
  ;[1 1 1] minion flow - chase and follow
  (if (!= (Utilities|Array|Length (Variables|Default|GetMinions)) 0)
    (Utilities|FlowControl|Sequence
      (:then_0
        (Variables|Default|SetBossPoint (Math|Vector|MakeVector _x _y 0.0)))
      (:then_1
        (Variables|Default|SetNumChaseMinion 0)
        (for (_array_element _array_index) (Variables|Default|GetMinions)
          ;;[1 1 1] chasing minion count
          (if (Variables|/Game/Minion/Blueprints/Minion_Actor.Minion_Actor_C|GetIsChasing _array_element)
            (Math|Integer|IncrementInt (Variables|Default|GetNumChaseMinion))))
        (Development|PrintString (Utilities|String|ToString(Integer) _array_index))
        (if (!= _array_index 0)
          (if (> (Variables|Default|GetNumChaseMinion) 0)
            ;;[1 1 1] player chasing
            (for _array_element_2 (Variables|Default|GetMinions)
              (if (not (Variables|/Game/Minion/Blueprints/Minion_Actor.Minion_Actor_C|GetIsKilled _array_element_2))
                (Utilities|FlowControl|Delay 1.0)
                (Transformation|SetWorldLocation (Variables|Default|GetMinionsTarget) (Math|Random|RandomPointinBoundingBox (Math|Vector|MakeVector _x_2 _y_2 0.0) (Variables|Default|GetRangeOfError)) false false)
                (bind _return (CallFunction|SetMaxForce _array_element_2))
                (bind _return_2 (CallFunction|SetMaxSpeed _return))
                (bind _return_3 (CallFunction|SetSepWeight _return_2))
                (bind _return_4 (CallFunction|SetAliWeight _return_3))
                (bind _return_5 (CallFunction|SetCohWeight _return_4))
                (bind _return_6 (CallFunction|SettoTargetWeight _return_5))
                (CallFunction|SetMaxTurnRate _return_6)))
            (else
              ;;[1 1 1] boss follow
              (for _array_element_3 (Variables|Default|GetMinions)
                (if (not (Variables|/Game/Minion/Blueprints/Minion_Actor.Minion_Actor_C|GetIsKilled _array_element_3))
                  (Utilities|FlowControl|Delay 3.0)
                  (Transformation|SetWorldLocation (Variables|Default|GetMinionsTarget) (Math|Random|RandomPointinBoundingBox (Variables|Default|GetBossPoint) (Variables|Default|GetRangeOfError)) false false)
                  (bind _return_7 (CallFunction|SetMaxForce _array_element_3))
                  (bind _return_8 (CallFunction|SetMaxSpeed _return_7))
                  (bind _return_9 (CallFunction|SetSepWeight _return_8))
                  (bind _return_10 (CallFunction|SetAliWeight _return_9))
                  (bind _return_11 (CallFunction|SetCohWeight _return_10))
                  (bind _return_12 (CallFunction|SettoTargetWeight _return_11))
                  (CallFunction|SetMaxTurnRate _return_12))))))))))

(fn ConstructionScript)

(fn SetMinionParameters
  (params (Minion :type Minion%20Actor%20Object%20Reference) (MaxForce :type Float%20%28single-precision%29) (MaxSpeed :type Float%20%28single-precision%29) (SepWeight :type Float%20%28single-precision%29) (AliWeight :type Float%20%28single-precision%29) (CohWeight :type Float%20%28single-precision%29) (ToTargetWeight :type Float%20%28single-precision%29) (MaxTurnRate :type Float%20%28single-precision%29))
  (Variables|/Game/Minion/Blueprints/Minion_Actor.Minion_Actor_C|SetMaxForce Minion MaxForce)
  (Variables|/Game/Minion/Blueprints/Minion_Actor.Minion_Actor_C|SetMaxSpeed Minion MaxSpeed)
  (Variables|/Game/Minion/Blueprints/Minion_Actor.Minion_Actor_C|SetSepWeight Minion SepWeight)
  (Variables|/Game/Minion/Blueprints/Minion_Actor.Minion_Actor_C|SetAliWeight Minion AliWeight)
  (Variables|/Game/Minion/Blueprints/Minion_Actor.Minion_Actor_C|SetCohWeight Minion CohWeight)
  (Variables|/Game/Minion/Blueprints/Minion_Actor.Minion_Actor_C|SetToTargetWeight Minion ToTargetWeight)
  (Variables|/Game/Minion/Blueprints/Minion_Actor.Minion_Actor_C|SetMaxTurnRate Minion MaxTurnRate)
  (Variables|/Game/Minion/Blueprints/Minion_Actor.Minion_Actor_C|SetMinionSpawnerRefarence Minion self))

(fn SetMaxForce
  (params (Minion :type Minion%20Actor%20Object%20Reference))
  (Variables|/Game/Minion/Blueprints/Minion_Actor.Minion_Actor_C|SetMaxForce Minion (Default|GetForceValue (Variables|Default|GetWID_Flocking)))
  (return Minion))

(fn SetMaxSpeed
  (params (Minion :type Minion%20Actor%20Object%20Reference))
  (Variables|/Game/Minion/Blueprints/Minion_Actor.Minion_Actor_C|SetMaxSpeed Minion (Default|GetSpeedValue (Variables|Default|GetWID_Flocking)))
  (return Minion))

(fn SetSepWeight
  (params (Minion :type Minion%20Actor%20Object%20Reference))
  (Variables|/Game/Minion/Blueprints/Minion_Actor.Minion_Actor_C|SetSepWeight Minion (Default|GetSepWeightValue (Variables|Default|GetWID_Flocking)))
  (return Minion))

(fn SetAliWeight
  (params (Minion :type Minion%20Actor%20Object%20Reference))
  (Variables|/Game/Minion/Blueprints/Minion_Actor.Minion_Actor_C|SetAliWeight Minion (Default|GetAliWeightValue (Variables|Default|GetWID_Flocking)))
  (return Minion))

(fn SetCohWeight
  (params (Minion :type Minion%20Actor%20Object%20Reference))
  (Variables|/Game/Minion/Blueprints/Minion_Actor.Minion_Actor_C|SetCohWeight Minion (Default|GetCohWeightValue (Variables|Default|GetWID_Flocking)))
  (return Minion))

(fn SettoTargetWeight
  (params (Minion :type Minion%20Actor%20Object%20Reference))
  (Variables|/Game/Minion/Blueprints/Minion_Actor.Minion_Actor_C|SetToTargetWeight Minion (Default|GettoTargetWeightValue (Variables|Default|GetWID_Flocking)))
  (return Minion))

(fn SetMaxTurnRate
  (params (Minion :type Minion%20Actor%20Object%20Reference))
  (return Minion))