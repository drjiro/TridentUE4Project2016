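; Stomp crack effect actor for the Wrath boss, a particle that travels in a straight line.
; On BeginPlay it records the crack particle's world location and sets a short lifespan.
; Each Tick it teleport-free moves the actor a fixed step along negative world Y without sweeping, so speed depends on frame rate.
; The overlap event is empty, so no hit logic runs here.
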(event EventBeginPlay
  (bind _output_get (Variables|Default|SetStartPosition (Transformation|GetWorldLocation (Variables|Default|GetCrackParticle))))
  (Variables|Default|SetCrackPillarLocation _output_get)
  (Actor|SetLifeSpan 5.0))

(event Collision|EventActorBeginOverlap
  (params (OtherActor :type Actor%20Object%20Reference)))

(event EventTick
  (params (DeltaSeconds :type Float%20%28single-precision%29))
  ;[1 1 1] Move effect
  (Transformation|SetActorLocation (Math|Vector|MakeVector (.X (Math|Vector|BreakVector (Variables|Default|GetCrackPillarLocation))) (+ (.Y (Math|Vector|BreakVector (Variables|Default|GetCrackPillarLocation))) -1e+01) (.Z (Math|Vector|BreakVector (Variables|Default|GetCrackPillarLocation)))) false false)
  (Variables|Default|SetCrackPillarLocation (Math|Vector|MakeVector (.X (Math|Vector|BreakVector (Variables|Default|GetCrackPillarLocation))) (+ (.Y (Math|Vector|BreakVector (Variables|Default|GetCrackPillarLocation))) -1e+01) (.Z (Math|Vector|BreakVector (Variables|Default|GetCrackPillarLocation))))))

(fn ConstructionScript)