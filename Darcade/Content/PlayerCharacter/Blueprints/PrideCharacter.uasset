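; Player character with stick-gesture melee combat, switchable sword, hammer and javelin, dash, enemy facing and pause.
; Right-stick angle and direction select swings, stabs or overheads in PrideAnimBlueprint; weapon end-overlap damages enemies for sword hits that avoid armor.
; Holding javelin zooms the camera and traces a target from Tick, with damage and effects on release.
; Enemy hits shatter health crystals and return the player to start, ending in game over.
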(event OnComponentEndOverlap(WeaponCollision)
  (params (OverlappedComponent :type Primitive%20Component%20Object%20Reference) (OtherActor :type Actor%20Object%20Reference) (OtherComp :type Primitive%20Component%20Object%20Reference) (OtherBodyIndex :type Integer))
  ;[1 1 1] Weapon hit
  (if (not (== OtherActor (Game|GetPlayerCharacter 0)))
    (bind _asai_enemy (Utilities|Casting|CastToAI_Enemy OtherActor))
    (if (Components|ComponentHasTag OtherComp "Armor")
      (Variables|Default|SetArmorHit? true)
      (elif (Variables|Default|GetArmorHit?)
        (Development|PrintString "Not!!!!!!!!!!!!!!!!HIT!!!!!!!!!!!!!!!!!!!!!!!!" :!label _label)
        (elif (Utilities|Enum|Equal(Enum) (Variables|Default|GetWeaponID) "NewEnumerator0")
          (if (== (Variables|/Game/AI/AI_Enemy.AI_Enemy_C|GetDamageCollision _asai_enemy) OtherComp)
            (Default|Damage _asai_enemy)
            (else
              (goto _label))))))))

(event Custom|ResetSpeed
  ;[1 1 1] Dash
  (Variables|/Script/Engine.CharacterMovementComponent|SetMaxWalkSpeed (Variables|Character|GetCharacterMovement) 6e+02)
  (Variables|Default|SetIsDashing false))

(event Custom|Die%20Timer
  ;[1 1 1] Health
  ;;[1 1 1] Respawn position
  (Variables|/Script/Engine.CharacterMovementComponent|SetDefaultLandMovementMode (Variables|Character|GetCharacterMovement) "MOVE_Walking")
  (Variables|Default|SetDie? false)
  (Transformation|SetActorLocation (Variables|Default|GetStartPosition) false false)
  (if (<= (Variables|Default|GetHealth) 0)
    (Variables|Default|SetHealth 0)
    ;[1 1 1] GameOver
    (Rendering|SetActorHiddenInGame true)
    (Collision|SetActorEnableCollision false)
    (bind _returnvalue (UserInterface|CreateWidget "/Game/ThirdPersonCPP/GameOverwidget.GameOverwidget_C"))
    (UserInterface|Viewport|AddtoViewport _returnvalue 0)))

(event Custom|GetHit
  (params (Hit :type Hit%20Result%20Structure%20%28by%20ref%29))
  ;[1 1 1] Health
  (if (not (Variables|Default|GetDie?))
    (if (Actor|ActorHasTag (.HitActor (Collision|BreakHitResult Hit)) "Enemy")
      (bind _output_get (Variables|Default|SetHealth (- (Variables|Default|GetHealth) 1)))
      ;;[1 1 1] Respawn position
      (CallFunction|CrystalDecrease _output_get)
      (Variables|Default|SetDie? true)
      (Variables|/Script/Engine.CharacterMovementComponent|SetDefaultLandMovementMode (Variables|Character|GetCharacterMovement) "MOVE_None")
      (Utilities|Time|SetTimerbyEvent (delegate Custom|Die%20Timer) 3.0))))

(event Collision|EventActorBeginOverlap
  (params (OtherActor :type Actor%20Object%20Reference)))

(event EventBeginPlay
  (Variables|Default|SetStartPosition (Transformation|GetActorLocation))
  (bind _outactors (Actor|GetAllActorsOfClass "/Game/Boss/Wrath/Blueprints/StompCrackBlueprint.StompCrackBlueprint_C"))
  (Variables|Default|SetStompCrackRef (Utilities|Array|Get(acopy) _outactors))
  (Collision|SetCollisionEnabled (Variables|Default|GetWeaponCollision) "NoCollision")
  (Collision|SetCollisionEnabled (Variables|Default|GetSword%20Mesh) "NoCollision")
  (Collision|SetCollisionEnabled (Variables|Default|GetHammer%20Mesh) "NoCollision"))

(event EventTick
  (params (DeltaSeconds :type Float%20%28single-precision%29))
  (bind _followcamera (Variables|Default|GetFollowCamera))
  (bind _charactermovement (Variables|Character|GetCharacterMovement))
  (bind _returnvalue (Transformation|GetWorldLocation _followcamera))
  (bind _returnvalue_2 (Transformation|GetWorldRotation _followcamera))
  (bind _returnvalue_3 (Math|Vector|GetForwardVector _returnvalue_2))
  (bind _returnvalue_4 (* _returnvalue_3 4000))
  (bind _returnvalue_5 (+ _returnvalue _returnvalue_4))
  (Pawn|Components|CharacterMovement|SetMovementMode _charactermovement (Variables|/Script/Engine.CharacterMovementComponent|GetDefaultLandMovementMode _charactermovement) 0)
  ;[1 1 1] Jevelin Target
  (if (Variables|Default|GetJeverin%20Frag)
    ;;[1 1 1] カメラの拡大
    (if (<= (Variables|Default|Getin%20Field%20Of%20View) 5e+01)
      _
      (else
        (Variables|Default|Setin%20Field%20Of%20View (- (Variables|Default|Getin%20Field%20Of%20View) 2.0))
        (CallFunction|CameraZoomUp)))
    (bind (_outhit _returnvalue_6) (Collision|LineTraceByChannel _returnvalue _returnvalue_5 "TraceTypeQuery1" false 0 "ForOneFrame"))
    (if _returnvalue_6
      (Variables|Default|SetJeverin%20Hit%20Actor (.HitActor (Collision|BreakHitResult _outhit)))
      (Variables|Default|SetJevein%20Hit%20Position (.Location (Collision|BreakHitResult _outhit)))
      (else
        (bind (_outhit_2 _returnvalue_7) (Class|KismetSystemLibrary|CapsuleTraceSingleforObjects _returnvalue _returnvalue_5 0.0 0.0 (Utilities|Array|MakeArray "ObjectTypeQuery3") false 0 "ForOneFrame" true))
        (if _returnvalue_7
          (Variables|Default|SetJeverin%20Hit%20Actor (.HitActor (Collision|BreakHitResult _outhit_2)))
          (Variables|Default|SetJevein%20Hit%20Position (.Location (Collision|BreakHitResult _outhit_2)))
          (else
            (Variables|Default|SetJeverin%20Hit%20Actor 0)
            (Variables|Default|SetJevein%20Hit%20Position "0, 0, 0")))))
    (else
      ;[1 1 1] カメラの縮小
      (if (>= (Variables|Default|Getin%20Field%20Of%20View) 9e+01)
        ;[1 1 1] Swing Flag
        (if (<= (stale Input|AxisEvents|InputAxisAttackX AxisValue) 0.0)
          (if (<= (stale Input|AxisEvents|InputAxisAttackY AxisValue) 0.0)
            (Variables|Default|SetIs%20HeavySwing%20Flag false)))
        ;[1 1 1] Lock On Target Enemy
        (Utilities|FlowControl|Gate true
          (:Exit
            (bind _outactors (Actor|GetAllActorsOfClass "/Game/AI/AI_Enemy.AI_Enemy_C"))
            (for _array_element _outactors
              (if (Actor|ActorHasTag _array_element "Enemy")
                (Pawn|SetControlRotation (Game|GetPlayerController 0) (Math|Rotator|MakeRotator (.roll (Math|Rotator|FindLookatRotation (Transformation|GetActorLocation) (Transformation|GetActorLocation _array_element))) 0.0 (.yaw (Math|Rotator|FindLookatRotation (Transformation|GetActorLocation) (Transformation|GetActorLocation _array_element)))))))))
        (else
          (Variables|Default|Setin%20Field%20Of%20View (+ (Variables|Default|Getin%20Field%20Of%20View) 2.0))
          (CallFunction|CameraZoomDown))))))

(event Input|ActionEvents|InputActionExitGame
  (params (Key :type Key%20Structure :default "AnyKey"))
  ;[1 1 1] Exit game
  (:Released
    (Development|ExecuteConsoleCommand "EXIT")))

(event Input|ActionEvents|InputActionChangeHummer
  (params (Key :type Key%20Structure :default "AnyKey"))
  ;[1 1 1] ChangeWeapon
  (:Pressed
    (bind _output_get (Variables|Default|SetWeaponID "NewEnumerator1"))
    (CallFunction|AttachWeapon _output_get (Variables|Default|GetOldWeaponMesh))))

(event Input|ActionEvents|InputActionChangeSword
  (params (Key :type Key%20Structure :default "AnyKey"))
  ;[1 1 1] ChangeWeapon
  (:Pressed
    (bind _output_get (Variables|Default|SetWeaponID "NewEnumerator0"))
    (CallFunction|AttachWeapon _output_get (Variables|Default|GetOldWeaponMesh))))

(event Input|ActionEvents|InputActionChangeJavelin
  (params (Key :type Key%20Structure :default "AnyKey"))
  (bind _jevein_hit_position (Variables|Default|GetJevein%20Hit%20Position))
  ;[1 1 1] ChangeWeapon
  (:Pressed
    (CallFunction|AttachWeapon "NewEnumerator2" (Variables|Default|GetOldWeaponMesh))
    (bind _aspride_anim_blueprint (Utilities|Casting|CastToPrideAnimBlueprint (Components|SkeletalMesh|GetAnimInstance (Variables|Character|GetMesh))))
    (Default|JavelinThrow _aspride_anim_blueprint)
    ;[1 1 1] jevelin Attack
    ;;[1 1 1] カメラの拡大
    (Variables|Default|SetJeverin%20Frag true)
    (Variables|Default|SetPlayer%20Rotation (Transformation|GetActorRotation)))
  (:Released
    (Utilities|FlowControl|Delay 0.5)
    (CallFunction|AttachWeapon (Variables|Default|GetWeaponID) (Variables|Default|GetJeveline%20Mesh))
    (bind _aspride_anim_blueprint_2 (Utilities|Casting|CastToPrideAnimBlueprint (Components|SkeletalMesh|GetAnimInstance (Variables|Character|GetMesh))))
    (Variables|/Game/PlayerCharacter/Animations/PrideAnimBlueprint.PrideAnimBlueprint_C|SetHolding%20Javelin _aspride_anim_blueprint_2 false)
    (if (Math|Vector|Equal(Vector) _jevein_hit_position "0, 0,0.000000" 0.0001)
      _
      (else
        (Utilities|FlowControl|Delay 0.5)
        (Effects|SpawnEmitteratLocation "/Game/Assets/Effects/FX_MainCharacter/P_JavelinHit.P_JavelinHit" _jevein_hit_position "0.000000, 0,90.000000")))
    ;;[1 1 1] カメラの縮小
    (Variables|Default|SetJeverin%20Frag false)
    ;;[1 1 1] Enemy Jevelin Damege
    (if (not (stale EventTick _returnvalue_6))
      (bind _asai_enemy (Utilities|Casting|CastToAI_Enemy (Variables|Default|GetJeverin%20Hit%20Actor)))
      (Default|Damage _asai_enemy))))

(event Input|ActionEvents|InputActionEnemyLock
  (params (Key :type Key%20Structure :default "AnyKey"))
  ;[1 1 1] Lock On Target Enemy
  (:Pressed
    (Utilities|FlowControl|FlipFlop
      (:A
        (Utilities|FlowControl|Gate true) ; enters at Open
      )
      (:B
        (Utilities|FlowControl|Gate true) ; enters at Close
      ))))

(event Input|ActionEvents|InputActionPause
  (params (Key :type Key%20Structure :default "AnyKey"))
  ;[1 1 1] Pause
  (:Pressed
    (Utilities|IsValid (Variables|Default|GetPauseMenuReference)
      (:Is%20Valid
        _)
      (:Is%20Not%20Valid
        (bind _returnvalue (UserInterface|CreateWidget "/Game/Menu/UIPauseMenu.UIPauseMenu_C"))
        (bind _output_get (Variables|Default|SetPauseMenuReference _returnvalue))))
    (Input|SetInputModeUIOnly (Game|GetPlayerController 0) (Variables|/Game/Menu/UIPauseMenu.UIPauseMenu_C|GetButtonMainReturnToGame _output_get) "DoNotLock")
    (UserInterface|Viewport|AddtoViewport _output_get 0)
    (Game|SetGamePaused true)))

(event Input|ActionEvents|InputActionGameOver
  (params (Key :type Key%20Structure :default "AnyKey"))
  (:Pressed
    (if (Variables|Default|GetbHidden)
      (Game|OpenLevel(byName) "LevelMainMenu"))))

(event Input|ActionEvents|InputActionGameClear
  (params (Key :type Key%20Structure :default "AnyKey"))
  (:Pressed
    (bind _outactors (Actor|GetAllActorsOfClass "/Game/AI/AI_Enemy.AI_Enemy_C"))
    (for _array_element _outactors
      (if (Actor|ActorHasTag _array_element "Enemy")
        (if (Variables|/Script/Engine.Actor|GetbHidden _array_element)
          (Game|OpenLevel(byName) "LevelMainMenu"))))))

(event Input|AxisEvents|InputAxisTurnRate
  (params (AxisValue :type Float%20%28single-precision%29))
  (if (not (Variables|Default|GetJeverin%20Frag))
    (Pawn|Input|AddControllerYawInput AxisValue)))

(event Input|AxisEvents|InputAxisAttackX
  (params (AxisValue :type Float%20%28single-precision%29))
  (bind _returnvalue (Utilities|Time|GetGameTimeinSeconds))
  (bind _weaponid (Variables|Default|GetWeaponID))
  (bind _weaponid_2 (Variables|Default|GetWeaponID))
  ;[1 1 1] Attack controls
  (if (not (Variables|Default|GetDie?))
    (if (or (!= AxisValue 0.0) (!= (stale Input|AxisEvents|InputAxisAttackY AxisValue) 0.0))
      (if (Variables|Default|GetJeverin%20Frag)
        (CallFunction|JeverinCameraMove (stale Input|AxisEvents|InputAxisAttackY AxisValue) AxisValue)
        (elif (== (+ (Class|KismetMathLibrary|DegAtan2 AxisValue (stale Input|AxisEvents|InputAxisAttackY AxisValue)) 1.8e+02) (Variables|Default|GetStick%20Angle)) ; Check if stick angle has changed
          ;;[1 1 1] Overhead attack
          (if (and (<= (Variables|Default|GetStick%20Angle) 209.0) (>= (Variables|Default|GetStick%20Angle) 151.0))
            (CallFunction|Overhead (and (<= (Variables|Default|GetStick%20Angle) 209.0) (>= (Variables|Default|GetStick%20Angle) 151.0)) _weaponid_2)
            (bind _output_get (Variables|Default|SetOverhead%20Time _returnvalue))
            (elif (or (< (Variables|Default|GetStick%20Angle) 2e+01) (> (Variables|Default|GetStick%20Angle) 3.4e+02))
              (if (<= (- _returnvalue _output_get) 0.07)
                (Collision|SetCollisionEnabled (Variables|Default|GetWeaponCollision) "QueryOnly")
                (bind _aspride_anim_blueprint (Utilities|Casting|CastToPrideAnimBlueprint (Components|SkeletalMesh|GetAnimInstance (Variables|Character|GetMesh))))
                (Default|EndOverhead _aspride_anim_blueprint (Animation|Montage|MontageIsPlaying _aspride_anim_blueprint 0)))
              (else
                ;[1 1 1] Stab
                (if (or (<= (stale _output_get_3) 15.0) (>= (stale _output_get_3) 345.0)) :!label _label
                  (CallFunction|Stab _weaponid)))))
          (else
            (bind _output_get_2 (Variables|Default|SetStick%20Angle%20Delta (- (+ (Class|KismetMathLibrary|DegAtan2 AxisValue (stale Input|AxisEvents|InputAxisAttackY AxisValue)) 1.8e+02) (Variables|Default|GetStick%20Angle))))
            (bind _output_get_3 (Variables|Default|SetStick%20Angle (+ (Class|KismetMathLibrary|DegAtan2 AxisValue (stale Input|AxisEvents|InputAxisAttackY AxisValue)) 1.8e+02)))
            (Development|PrintText (Utilities|Text|ToText(Float) _output_get_3 "HalfToEven") true true "(R=0.000000,G=0.660000,B=1.000000,A=1.000000)" 1.0)
            (if (>= _output_get_3 2.1e+02)
              (if (and (<= _output_get_3 2.6e+02) (>= _output_get_3 2.1e+02)) ; Check stick start position
                ;;[1 1 1] Swing Left
                (CallFunction|HeavySwingLeft (> _output_get_2 0.0) _weaponid)
                (elif (and (<= _output_get_3 3.3e+02) (>= _output_get_3 2.6e+02))
                  (if (not (Variables|Default|GetIs%20HeavySwing%20Flag))
                    (CallFunction|LightSwingLeft (> _output_get_2 0.0) _weaponid)
                    (Development|PrintString "Lighttttttttttttttttttttttttttttttttttttttttttttt"))
                  (else
                    (goto _label))))
              (else
                ;;[1 1 1] Swing Right
                (if (and (<= _output_get_3 1.5e+02) (>= _output_get_3 1e+02))
                  (CallFunction|HeavySwingRight (< _output_get_2 0.0) _weaponid_2)
                  (elif (and (<= _output_get_3 99.0) (>= _output_get_3 3e+01))
                    (if (not (Variables|Default|GetIs%20HeavySwing%20Flag))
                      (CallFunction|LightSwingRight (< _output_get_2 0.0) _weaponid_2)
                      (Development|PrintString "Lighttttttttttttttttttttttttttttttttttttttttttttt"))))))))))))

(event Input|AxisEvents|InputAxisAttackY
  (params (AxisValue :type Float%20%28single-precision%29))
  ;[1 1 1] Attack controls
)

(event Input|GamepadEvents|GamepadFaceButtonBottom
  (params (Key :type Key%20Structure :default "AnyKey"))
  (bind _charactermovement (Variables|Character|GetCharacterMovement))
  ;[1 1 1] Dash
  (:Pressed
    (Variables|Default|SetIsButtonA true)
    (if (not (Variables|Default|GetIsDashing))
      (Variables|Default|SetIsDashing true)
      (Variables|/Script/Engine.CharacterMovementComponent|SetMaxWalkSpeed _charactermovement (* (Class|MovementComponent|GetMaxSpeed _charactermovement) 1.5e+02))
      (Utilities|Time|SetTimerbyEvent (delegate Custom|ResetSpeed) 0.5)))
  (:Released
    (Variables|Default|SetIsButtonA false)))

(event Input|KeyboardEvents|L
  (params (Key :type Key%20Structure :default "AnyKey"))
  ;[1 1 1] Test spawn crack effect
  (:Pressed
    (Utilities|FlowControl|DoOnce false :!label _label
      (:Completed
        (Game|SpawnActorfromClass "/Game/Boss/Wrath/Blueprints/StompCrackBlueprint.StompCrackBlueprint_C" (Transformation|GetWorldTransform (Variables|Character|GetMesh)) "Undefined" 0 0))))
  (:Released
    (goto _label Reset)))

(event Input|GamepadEvents|GamepadRightStickUp
  (params (Key :type Key%20Structure :default "AnyKey"))
  ;[1 1 1] Attack controls
  ;;[1 1 1] End overhead attack
  (:Pressed
    (bind _aspride_anim_blueprint (Utilities|Casting|CastToPrideAnimBlueprint (Components|SkeletalMesh|GetAnimInstance (Variables|Character|GetMesh))))
    (Default|EndOverhead _aspride_anim_blueprint (Animation|Montage|MontageIsPlaying _aspride_anim_blueprint 0))))

(fn ConstructionScript
  (bind _weaponcollision (Variables|Default|GetWeaponCollision))
  (bind _weapon_mesh (Variables|Default|GetWeapon%20Mesh))
  (bind _weapon_mesh_2 (Variables|Default|GetWeapon%20Mesh))
  (bind _weapon_mesh_3 (Variables|Default|GetWeapon%20Mesh))
  ;[1 1 1] すべての武器を予め生成する
  ;;[1 1 1] ハンマー を生成する
  (CallFunction|CreateHammerWeapon "/Game/PlayerCharacter/Mesh/Weapons/hammer.hammer")
  (Rendering|SetVisibility _weapon_mesh false false)
  (bind _output_get (Variables|Default|SetHammer%20Mesh _weapon_mesh))
  ;;[1 1 1] 剣を生成する
  (CallFunction|CreateSwordWeapon "/Game/PlayerCharacter/Mesh/Weapons/sword.sword")
  (Rendering|SetVisibility _weapon_mesh_2 true false)
  (bind _output_get_2 (Variables|Default|SetSword%20Mesh _weapon_mesh_2))
  (Variables|Default|SetOldWeaponMesh _output_get_2)
  ;;[1 1 1] 槍を生成する
  (CallFunction|CreateJavelinWeapon "/Game/PlayerCharacter/Mesh/Weapons/SM_Spear.SM_Spear")
  (Rendering|SetVisibility _weapon_mesh_3 false false)
  (Variables|Default|SetJeveline%20Mesh _weapon_mesh_3)
  ;[1 1 1] Create Collision Box
  (Class|SceneComponent|Attachto _weaponcollision _output_get "SwordSocket" "KeepRelativeOffset" true)
  (Transformation|SetRelativeScale3D _weaponcollision (Variables|Default|GetSword%20Collision%20Scale))
  (Transformation|SetRelativeLocation (Variables|Default|GetWeaponCollision) "-70.000000,-55.000000,300.000000" false false)
  (Transformation|SetRelativeRotation (Variables|Default|GetWeaponCollision) "13.000000, 0,-10.000000" false false))

(fn CreateHammerWeapon
  (params (Hammer%20Mesh :type Static%20Mesh%20Object%20Reference))
  ;[1 1 1] create Skeletal Mesh
  (bind _returnvalue (AddComponent|AddStaticMeshComponent false))
  (Components|StaticMesh|SetStaticMesh _returnvalue Hammer%20Mesh)
  (Class|SceneComponent|Attachto _returnvalue (Variables|Character|GetMesh) "HammerSocket" "KeepRelativeOffset" true)
  (Variables|Default|SetWeapon%20Mesh _returnvalue))

(fn AttachWeapon
  (params (WeaponID :type WeaponList%20Enum) (OldWeapon :type Static%20Mesh%20Component%20Object%20Reference))
  (bind _hammer_mesh (Variables|Default|GetHammer%20Mesh))
  (bind _sword_mesh (Variables|Default|GetSword%20Mesh))
  ;[1 1 1] 手持ちの武器を非表示にする
  (Rendering|SetVisibility OldWeapon false false)
  (bind _aspride_anim_blueprint (Utilities|Casting|CastToPrideAnimBlueprint (Components|SkeletalMesh|GetAnimInstance (Variables|Character|GetMesh))))
  (Variables|/Game/PlayerCharacter/Animations/PrideAnimBlueprint.PrideAnimBlueprint_C|SetActive%20Weapon _aspride_anim_blueprint WeaponID)
  (switch Utilities|FlowControl|Switch|SwitchonWeaponList WeaponID
    (:NewEnumerator0
      ;[1 1 1] 武器を表示させる
      (Rendering|SetVisibility _sword_mesh true false)
      ;[1 1 1] 当たり判定の大きさ変更
      (Transformation|SetRelativeScale3D (Variables|Default|GetWeaponCollision) (Variables|Default|GetSword%20Collision%20Scale))
      (Variables|Default|SetOldWeaponMesh _sword_mesh)
      (Transformation|SetRelativeLocation (Variables|Default|GetWeaponCollision) "-70.000000,-55.000000,300.000000" false false)
      (Transformation|SetRelativeRotation (Variables|Default|GetWeaponCollision) "13.000000, 0,-10.000000" false false))
    (:NewEnumerator1
      (Rendering|SetVisibility _hammer_mesh true false)
      (Transformation|SetRelativeScale3D (Variables|Default|GetWeaponCollision) (Variables|Default|GetHummer%20Collision%20Scale))
      (Variables|Default|SetOldWeaponMesh _hammer_mesh)
      (Transformation|SetRelativeLocation (Variables|Default|GetWeaponCollision) "-30.000000,0.000000,350.000000" false false)
      (Transformation|SetRelativeRotation (Variables|Default|GetWeaponCollision) "10.000000, 0,0.000000" false false))
    (:NewEnumerator2
      (Rendering|SetVisibility (Variables|Default|GetJeveline%20Mesh) true false))))

(fn CameraZoomUp
  (bind _in_field_of_view (Variables|Default|GetIn%20Field%20Of%20View))
  (bind _followcamera (Variables|Default|GetFollowCamera))
  (Camera|SetFieldOfView _followcamera _in_field_of_view)
  (Transformation|SetRelativeLocation _followcamera (Math|Vector|MakeVector 0.0 _in_field_of_view _in_field_of_view) false false)
  (Transformation|SetActorRotation (Game|GetPlayerCharacter 0) (Math|Rotator|MakeRotator 0.0 0.0 (.yaw (Transformation|GetWorldRotation (Variables|Default|GetFollowCamera))))))

(fn HeavySwingLeft
  (params (Continue? :type Boolean) (Weapon%20ID :type WeaponList%20Enum))
  (Variables|Default|SetIs%20HeavySwing%20Flag true)
  (if (Utilities|Enum|Equal(Enum) Weapon%20ID "NewEnumerator0")
    (Collision|SetCollisionEnabled (Variables|Default|GetWeaponCollision) "QueryOnly" :!label _label)
    (bind _aspride_anim_blueprint (Utilities|Casting|CastToPrideAnimBlueprint (Components|SkeletalMesh|GetAnimInstance (Variables|Character|GetMesh))))
    (Default|Overhead _aspride_anim_blueprint Continue? Weapon%20ID)
    (elif (Utilities|Enum|Equal(Enum) Weapon%20ID "NewEnumerator1")
      (goto _label))))

(fn LightSwingLeft
  (params (Continue? :type Boolean) (Weapon%20ID :type WeaponList%20Enum))
  (Collision|SetCollisionEnabled (Variables|Default|GetWeaponCollision) "QueryOnly")
  (bind _aspride_anim_blueprint (Utilities|Casting|CastToPrideAnimBlueprint (Components|SkeletalMesh|GetAnimInstance (Variables|Character|GetMesh))))
  (Default|SwingLeft _aspride_anim_blueprint Continue? Weapon%20ID))

(fn HeavySwingRight
  (params (Continue? :type Boolean) (Weapon%20ID :type WeaponList%20Enum))
  (Variables|Default|SetIs%20HeavySwing%20Flag true)
  (Collision|SetCollisionEnabled (Variables|Default|GetWeaponCollision) "QueryOnly")
  (bind _aspride_anim_blueprint (Utilities|Casting|CastToPrideAnimBlueprint (Components|SkeletalMesh|GetAnimInstance (Variables|Character|GetMesh))))
  (Default|SwingRight _aspride_anim_blueprint Continue? Weapon%20ID))

(fn LightSwingRight
  (params (Continue? :type Boolean) (Weapon%20ID :type WeaponList%20Enum))
  (Collision|SetCollisionEnabled (Variables|Default|GetWeaponCollision) "QueryOnly")
  (bind _aspride_anim_blueprint (Utilities|Casting|CastToPrideAnimBlueprint (Components|SkeletalMesh|GetAnimInstance (Variables|Character|GetMesh))))
  (Default|SwingRight _aspride_anim_blueprint Continue? Weapon%20ID))

(fn Overhead
  (params (Continue? :type Boolean) (Weapon%20ID :type WeaponList%20Enum))
  (bind _aspride_anim_blueprint (Utilities|Casting|CastToPrideAnimBlueprint (Components|SkeletalMesh|GetAnimInstance (Variables|Character|GetMesh))))
  (Default|Overhead _aspride_anim_blueprint Continue? Weapon%20ID))

(fn Stab
  (params (Weapon%20ID :type WeaponList%20Enum))
  (Collision|SetCollisionEnabled (Variables|Default|GetWeaponCollision) "QueryOnly")
  (bind _aspride_anim_blueprint (Utilities|Casting|CastToPrideAnimBlueprint (Components|SkeletalMesh|GetAnimInstance (Variables|Character|GetMesh))))
  (Default|Stab _aspride_anim_blueprint Weapon%20ID))

(fn JeverinCameraMove
  (params (Camera%20RotationY :type Float%20%28single-precision%29) (Camera%20RotationZ :type Float%20%28single-precision%29))
  (Pawn|Input|AddControllerYawInput Camera%20RotationZ)
  (if (<= (.pitch (Variables|Default|GetCamera%20Rotation)) -3e+01)
    (if (not (<= Camera%20RotationY -0.1))
      (Variables|Default|SetCamera%20Rotation (Math|Rotator|MakeRotator 0.0 (+ Camera%20RotationY (.pitch (Variables|Default|GetCamera%20Rotation))) (+ Camera%20RotationZ (.yaw (Variables|Default|GetCamera%20Rotation)))) :!label _label)
      (Transformation|SetActorRotation (Math|Rotator|MakeRotator 0.0 0.0 (.yaw (Transformation|GetWorldRotation (Variables|Default|GetFollowCamera))))))
    (elif (>= (.pitch (Variables|Default|GetCamera%20Rotation)) 3e+01)
      (if (not (>= Camera%20RotationY 0.1))
        (goto _label))
      (else
        (Pawn|Input|AddControllerPitchInput Camera%20RotationY)
        (goto _label)))))

(fn CameraZoomDown
  (bind _in_field_of_view (Variables|Default|GetIn%20Field%20Of%20View))
  (bind _followcamera (Variables|Default|GetFollowCamera))
  (Camera|SetFieldOfView _followcamera _in_field_of_view)
  (Transformation|SetRelativeLocation _followcamera (Math|Vector|MakeVector 0.0 _in_field_of_view _in_field_of_view) false false)
  (Pawn|Input|AddControllerPitchInput (* (.pitch (Variables|Default|GetCamera%20Rotation)) -1.0))
  (Transformation|SetActorRotation (Game|GetPlayerCharacter 0) (Math|Rotator|MakeRotator 0.0 0.0 (.yaw (Transformation|GetWorldRotation (Variables|Default|GetFollowCamera)))))
  (Variables|Default|SetCamera%20Rotation "0, 0, 0"))

(fn CreateSwordWeapon
  (params (Sword%20Mesh :type Static%20Mesh%20Object%20Reference))
  ;[1 1 1] create Skeletal Mesh
  (bind _returnvalue (AddComponent|AddStaticMeshComponent false))
  (Components|StaticMesh|SetStaticMesh _returnvalue Sword%20Mesh)
  (Class|SceneComponent|Attachto _returnvalue (Variables|Character|GetMesh) "SwordSocket" "KeepRelativeOffset" true)
  (Variables|Default|SetWeapon%20Mesh _returnvalue)
  (Transformation|SetRelativeScale3D (Variables|Default|GetWeaponCollision) (Variables|Default|GetSword%20Collision%20Scale)))

(fn CreateJavelinWeapon
  (params (Javelin%20Mesh :type Static%20Mesh%20Object%20Reference))
  ;[1 1 1] create Skeletal Mesh
  (bind _returnvalue (AddComponent|AddStaticMeshComponent false))
  (Components|StaticMesh|SetStaticMesh _returnvalue Javelin%20Mesh)
  (Class|SceneComponent|Attachto _returnvalue (Variables|Character|GetMesh) "JavelinSocket" "KeepRelativeOffset" true)
  (Variables|Default|SetWeapon%20Mesh _returnvalue))

(fn CrystalDecrease
  (params (Health :type Integer))
  (bind _crystal3 (Variables|Default|GetCrystal3))
  (bind _crystal2 (Variables|Default|GetCrystal2))
  (bind _crystal1 (Variables|Default|GetCrystal1))
  (if (== Health 3)
    (Effects|SpawnEmitteratLocation "/Game/Assets/Effects/FX_MainCharacter/P_CrystalExplode.P_CrystalExplode" (Transformation|GetSocketLocation _crystal1 "None") "0.000000, 0,0.000000")
    (Components|DestroyComponent _crystal1)
    (elif (== Health 2)
      (Effects|SpawnEmitteratLocation "/Game/Assets/Effects/FX_MainCharacter/P_CrystalExplode.P_CrystalExplode" (Transformation|GetSocketLocation _crystal3 "None") "0.000000, 0,0.000000")
      (Components|DestroyComponent _crystal3)
      (elif (== Health 1)
        (Effects|SpawnEmitteratLocation "/Game/Assets/Effects/FX_MainCharacter/P_CrystalExplode.P_CrystalExplode" (Transformation|GetSocketLocation _crystal2 "None") "0.000000, 0,0.000000")
        (Components|DestroyComponent _crystal2)))))