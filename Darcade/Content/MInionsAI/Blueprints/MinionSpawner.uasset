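; Spawner actor that creates a flock of minions in a box around the player and steers them through a shared, hidden target component.
; On BeginPlay each minion receives that target and initial flocking parameters.
; Every tick the target snaps to the player while IsChasing, otherwise to the spawner.
; Each tick also copies live force, speed and steering weights from the WID_Flocking widget to every minion; SetMaxTurnRate changes nothing.
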(event EventBeginPlay
  (Rendering|SetVisibility (Variables|Default|GetMinionsTarget) false false)
  (bind _foundwidgets (Widget|GetAllWidgetsOfClass "/Game/MInionsAI/Blueprints/WID_Flocking.WID_Flocking_C" true))
  (Variables|Default|SetWID_Flocking (Utilities|Array|Get(acopy) _foundwidgets))
  (for _index (range 0 (Variables|Default|GetNumSpawnMinion))
    (bind _returnvalue (Game|SpawnActorfromClass "/Game/MInionsAI/Blueprints/Minion.Minion_C" (Math|Transform|MakeTransform (Math|Random|RandomPointinBoundingBox (Transformation|GetActorLocation (Game|GetPlayerCharacter 0)) (Variables|Default|GetSpawnBoxSize)) "0, 0, 0" (Variables|Default|GetMinionScale)) "Undefined" 0 0))
    (Utilities|Array|AddUnique (Variables|Default|GetMinions) _returnvalue)
    (Variables|/Game/MInionsAI/Blueprints/Minion.Minion_C|SetTarget _returnvalue (Variables|Default|GetMinionsTarget))
    (CallFunction|SetMinionParameters _returnvalue (Variables|Default|GetMaxForce) (Variables|Default|GetMaxSpeed) (Variables|Default|GetSepWeight) (Variables|Default|GetAliWeight) (Variables|Default|GetCohWeight) (Variables|Default|GetToTargetWeight) (Variables|Default|GetMaxTurnRate)))
  (Transformation|SetWorldLocation (Variables|Default|GetMinionsTarget) (Transformation|GetActorLocation) false false))

(event EventTick
  (params (DeltaSeconds :type Float%20%28single-precision%29))
  (if (Variables|Default|GetIsChasing)
    (Utilities|FlowControl|Sequence
      (:then_0
        (Transformation|SetWorldLocation (Variables|Default|GetMinionsTarget) (Transformation|GetActorLocation (Game|GetPlayerCharacter 0)) false false))
      (:then_1
        (for _array_element (Variables|Default|GetMinions)
          (bind _return (CallFunction|SetMaxForce _array_element))
          (bind _return_2 (CallFunction|SetMaxSpeed _return))
          (bind _return_3 (CallFunction|SetSepWeight _return_2))
          (bind _return_4 (CallFunction|SetAliWeight _return_3))
          (bind _return_5 (CallFunction|SetCohWeight _return_4))
          (bind _return_6 (CallFunction|SettoTargetWeight _return_5))
          (CallFunction|SetMaxTurnRate _return_6))))
    (else
      (Utilities|FlowControl|Sequence
        (:then_0
          (Transformation|SetWorldLocation (Variables|Default|GetMinionsTarget) (Transformation|GetActorLocation) false false))
        (:then_1
          (for _array_element_2 (Variables|Default|GetMinions)
            (bind _return_7 (CallFunction|SetMaxForce _array_element_2))
            (bind _return_8 (CallFunction|SetMaxSpeed _return_7))
            (bind _return_9 (CallFunction|SetSepWeight _return_8))
            (bind _return_10 (CallFunction|SetAliWeight _return_9))
            (bind _return_11 (CallFunction|SetCohWeight _return_10))
            (bind _return_12 (CallFunction|SettoTargetWeight _return_11))
            (CallFunction|SetMaxTurnRate _return_12)))))))

(fn ConstructionScript)

(fn SetMinionParameters
  (params (Minion :type Minion%20Object%20Reference) (MaxForce :type Float%20%28single-precision%29) (MaxSpeed :type Float%20%28single-precision%29) (SepWeight :type Float%20%28single-precision%29) (AliWeight :type Float%20%28single-precision%29) (CohWeight :type Float%20%28single-precision%29) (ToTargetWeight :type Float%20%28single-precision%29) (MaxTurnRate :type Float%20%28single-precision%29))
  (Variables|/Game/MInionsAI/Blueprints/Minion.Minion_C|SetMaxForce Minion MaxForce)
  (Variables|/Game/MInionsAI/Blueprints/Minion.Minion_C|SetMaxSpeed Minion MaxSpeed)
  (Variables|/Game/MInionsAI/Blueprints/Minion.Minion_C|SetSepWeight Minion SepWeight)
  (Variables|/Game/MInionsAI/Blueprints/Minion.Minion_C|SetAliWeight Minion AliWeight)
  (Variables|/Game/MInionsAI/Blueprints/Minion.Minion_C|SetCohWeight Minion CohWeight)
  (Variables|/Game/MInionsAI/Blueprints/Minion.Minion_C|SetToTargetWeight Minion ToTargetWeight)
  (Variables|/Game/MInionsAI/Blueprints/Minion.Minion_C|SetMaxTurnRate Minion MaxTurnRate))

(fn SetMaxForce
  (params (Minion :type Minion%20Object%20Reference))
  (Variables|/Game/MInionsAI/Blueprints/Minion.Minion_C|SetMaxForce Minion (Default|GetForceValue (Variables|Default|GetWID_Flocking)))
  (return Minion))

(fn SetMaxSpeed
  (params (Minion :type Minion%20Object%20Reference))
  (Variables|/Game/MInionsAI/Blueprints/Minion.Minion_C|SetMaxSpeed Minion (Default|GetSpeedValue (Variables|Default|GetWID_Flocking)))
  (return Minion))

(fn SetSepWeight
  (params (Minion :type Minion%20Object%20Reference))
  (Variables|/Game/MInionsAI/Blueprints/Minion.Minion_C|SetSepWeight Minion (Default|GetSepWeightValue (Variables|Default|GetWID_Flocking)))
  (return Minion))

(fn SetAliWeight
  (params (Minion :type Minion%20Object%20Reference))
  (Variables|/Game/MInionsAI/Blueprints/Minion.Minion_C|SetAliWeight Minion (Default|GetAliWeightValue (Variables|Default|GetWID_Flocking)))
  (return Minion))

(fn SetCohWeight
  (params (Minion :type Minion%20Object%20Reference))
  (Variables|/Game/MInionsAI/Blueprints/Minion.Minion_C|SetCohWeight Minion (Default|GetCohWeightValue (Variables|Default|GetWID_Flocking)))
  (return Minion))

(fn SettoTargetWeight
  (params (Minion :type Minion%20Object%20Reference))
  (Variables|/Game/MInionsAI/Blueprints/Minion.Minion_C|SetToTargetWeight Minion (Default|GettoTargetWeightValue (Variables|Default|GetWID_Flocking)))
  (return Minion))

(fn SetMaxTurnRate
  (params (Minion :type Minion%20Object%20Reference))
  (return Minion))