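; Boid actor that flocks with nearby Boids while steering toward a Target.
; Each tick a sphere overlap finds neighbors, and weighted separation, alignment and cohesion forces accumulate into acceleration.
; Velocity restarts from the weighted target direction, adds acceleration, and is mirrored when a forward trace hits WorldStatic.
; Velocity only sets heading through interpolated rotation, with a separate wall-avoid turn rate, while movement is a fixed forward step per frame.
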(event EventActorBeginOverlap
  (params (OtherActor :type Actor%20Object%20Reference)))

(event EventTick
  (params (DeltaSeconds :type Float%20%28single-precision%29))
  (Variables|Default|SetDeltaTime DeltaSeconds)
  (bind _outactors (Class|KismetSystemLibrary|SphereOverlapActorsNEW (Transformation|GetActorLocation) (Variables|/Script/Engine.SphereComponent|GetSphereRadius (Variables|Default|GetSphere)) (Utilities|Array|MakeArray "ObjectTypeQuery2") "Boid_C" (Utilities|Array|MakeArray self)))
  (CallFunction|Flock _outactors)
  (Variables|Default|SetVelocity (* (Math|Vector|Normalize (- (Transformation|GetWorldLocation (Variables|Default|GetTarget)) (Transformation|GetActorLocation))) (Variables|OpenParam|GetToTargetWeight)))
  (CallFunction|Update))

(event EventBeginPlay)

(fn ConstructionScript)

(fn Flock
  (params (boids :type Array%20of%20Actor%20Object%20References))
  (bind _return (CallFunction|Separate boids))
  (LocalVariables|SetSep _return)
  (bind _return_2 (CallFunction|Align boids))
  (LocalVariables|SetAli _return_2)
  (bind _return_3 (CallFunction|Cohesion boids))
  (LocalVariables|SetCoh _return_3)
  (CallFunction|ApplyForce (* (LocalVariables|GetSep) (Variables|OpenParam|GetSepWeight)))
  (CallFunction|ApplyForce (* (LocalVariables|GetAli) (Variables|OpenParam|GetAliWeight)))
  (CallFunction|ApplyForce (* (LocalVariables|GetCoh) (Variables|OpenParam|GetCohWeight))))

(fn Update
  (bind _returnvalue (Transformation|GetActorLocation))
  (bind _output_get (Variables|Default|SetVelocity (+ (Variables|Default|GetVelocity) (Variables|Default|GetAcceleration))))
  (Variables|Default|SetVelocity (Math|Vector|ClampVectorSize _output_get 0.0 (Variables|OpenParam|GetMaxSpeed)))
  (bind (_outhit _returnvalue_2) (Collision|LineTraceForObjects (Transformation|GetActorLocation) (+ (Transformation|GetActorLocation) (* (Transformation|GetActorForwardVector) 1e+03)) (Utilities|Array|MakeArray "ObjectTypeQuery1") false 0 "None"))
  (if _returnvalue_2
    (Variables|Default|SetVelocity (Math|Vector|MirrorVectorbyNormal (.location _outhit) (.impactnormal _outhit)))
    (LocalVariables|SetRateIndex 1)
    (else
      (LocalVariables|SetRateIndex 0)))
  (Transformation|SetActorRotation (Math|Interpolation|RInterpTo (Transformation|GetActorRotation) (Math|Rotator|FindLookatRotation _returnvalue (+ _returnvalue (Variables|Default|GetVelocity))) (Variables|Default|GetDeltaTime) (Utilities|Select :Index (LocalVariables|GetRateIndex) :Option%200 (Variables|OpenParam|GetMaxTurnRate) :Option%201 (LocalVariables|GetWallAvoidTurnRate))))
  (Transformation|AddActorLocalOffset (Math|Vector|MakeVector 1e+01 0.0 0.0) false false)
  (Variables|Default|SetAcceleration (* (Variables|Default|GetAcceleration) 0.0)))

(fn ApplyForce
  (params (force :type Vector))
  (Variables|Default|SetAcceleration (+ (Variables|Default|GetAcceleration) force)))

(fn Separate
  (params (boids :type Array%20of%20Actor%20Object%20References))
  ;[1 1 1] 分離行動
  (for _array_element boids
    (LocalVariables|SetOther _array_element)
    (if (and (> (Math|Vector|VectorLength (- (Transformation|GetActorLocation) (Transformation|GetActorLocation _array_element))) 0.0) true)
      (LocalVariables|SetSteer (+ (LocalVariables|GetSteer) (/ (Math|Vector|Normalize (- (Transformation|GetActorLocation) (Transformation|GetActorLocation (LocalVariables|GetOther)))) (Math|Vector|VectorLength (- (Transformation|GetActorLocation) (Transformation|GetActorLocation (LocalVariables|GetOther)))))))
      (Math|Integer|IncrementInt (LocalVariables|GetCount))))
  (if (> (LocalVariables|GetCount) 0)
    (bind _output_get (LocalVariables|SetSteer (/ (LocalVariables|GetSteer) (Math|Conversions|ToFloat(Integer) (LocalVariables|GetCount)))))
    (if (> (Math|Vector|VectorLength _output_get) 0.0)
      (return (Math|Vector|ClampVectorSize (- (Math|Vector|Normalize (LocalVariables|GetSteer)) (Variables|Default|GetVelocity)) 0.0 (Variables|OpenParam|GetMaxForce)))
      (else
        _)))
  (return "0, 0, 0"))

(fn Align
  (params (boids :type Array%20of%20Actor%20Object%20References))
  ;[1 1 1] 整列行動
  (for _array_element boids
    (if (and (> (Math|Vector|VectorLength (- (Transformation|GetActorLocation) (Transformation|GetActorLocation _array_element))) 0.0) true)
      (LocalVariables|SetSum (+ (LocalVariables|GetSum) (Transformation|GetVelocity _array_element)))
      (Math|Integer|IncrementInt (LocalVariables|GetCount))))
  (if (> (LocalVariables|GetCount) 0)
    (bind _output_get (LocalVariables|SetSum (/ (LocalVariables|GetSum) (Math|Conversions|ToFloat(Integer) (LocalVariables|GetCount)))))
    (return (Math|Vector|ClampVectorSize (- (* (Math|Vector|Normalize _output_get) (Variables|OpenParam|GetMaxSpeed)) (Variables|Default|GetVelocity)) 0.0 (Variables|OpenParam|GetMaxForce)))
    (else
      (return "0, 0, 0"))))

(fn Cohesion
  (params (boids :type Array%20of%20Actor%20Object%20References))
  ;[1 1 1] 結合行動
  (for _array_element boids
    (if (and (> (Math|Vector|VectorLength (- (Transformation|GetActorLocation) (Transformation|GetActorLocation _array_element))) 0.0) true)
      (LocalVariables|SetSum (+ (LocalVariables|GetSum) (Transformation|GetActorLocation _array_element)))
      (Math|Integer|IncrementInt (LocalVariables|GetCount))))
  (if (> (LocalVariables|GetCount) 0)
    (bind _output_get (LocalVariables|SetSum (/ (LocalVariables|GetSum) (Math|Conversions|ToFloat(Integer) (LocalVariables|GetCount)))))
    (bind _return (CallFunction|Seek _output_get))
    (return _return)
    (else
      (return "0, 0, 0"))))

(fn Seek
  (params (target :type Vector))
  (return (Math|Vector|ClampVectorSize (- (* (Math|Vector|Normalize (- target (Transformation|GetActorLocation))) (Variables|OpenParam|GetMaxSpeed)) (Variables|Default|GetVelocity)) 0.0 (Variables|OpenParam|GetMaxForce))))