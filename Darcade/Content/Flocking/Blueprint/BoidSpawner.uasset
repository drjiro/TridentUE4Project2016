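; Actor that spawns a flock of boids at random points in a box and gives them a shared, wandering target.
; BeginPlay sets each boid's initial force, speed, turn rate and steering weights, then caches the WID_Flocking widget for tuning.
; Tick relocates the target randomly about every five seconds via a Delay and pushes widget values to every boid each frame.
; SetMaxTurnRate is an empty pass-through, so turn rate stays at its spawn value.
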(event EventBeginPlay
  (bind _movetarget (Variables|Default|GetMoveTarget))
  (bind _foundwidgets (Widget|GetAllWidgetsOfClass "/Game/Flocking/Blueprint/WID_Flocking.WID_Flocking_C" true))
  (bind _aswid_flocking (Utilities|Casting|CastToWID_Flocking (Utilities|Array|Get(acopy) _foundwidgets)))
  (Variables|Default|SetWID_Flocking _aswid_flocking)
  (for _index (range 0 (Variables|Default|GetNumSpawnBoid))
    (bind _returnvalue (Game|SpawnActorfromClass "/Game/Flocking/Blueprint/Boid.Boid_C" (Math|Transform|MakeTransform (Math|Random|RandomPointinBoundingBox (Transformation|GetActorLocation) (Variables|Default|GetSpawnBoxSize)) "0, 0, 0" (Variables|Default|GetBoidScale)) "Undefined" 0 0))
    (Utilities|Array|AddUnique (Variables|Default|GetBoids) _returnvalue)
    (Variables|/Game/Flocking/Blueprint/Boid.Boid_C|SetTarget _returnvalue (Variables|Default|GetBoidsTarget))
    (CallFunction|SetBoidParameters _returnvalue (Variables|Default|GetMaxForce) (Variables|Default|GetMaxSpeed) (Variables|Default|GetSepWeight) (Variables|Default|GetAliWeight) (Variables|Default|GetCohWeight) (Variables|Default|GetToTargetWeight) (Variables|Default|GetMaxTurnRate)))
  (Transformation|SetWorldLocation (Variables|Default|GetBoidsTarget) (+ (Math|Random|RandomPointinBoundingBox (Transformation|GetActorLocation) _movetarget) _movetarget) false false))

(event EventTick
  (params (DeltaSeconds :type Float%20%28single-precision%29))
  (bind _movetarget (Variables|Default|GetMoveTarget))
  (Utilities|FlowControl|Sequence
    (:then_0
      (Utilities|FlowControl|Delay 5.0)
      (Transformation|SetWorldLocation (Variables|Default|GetBoidsTarget) (+ (Math|Random|RandomPointinBoundingBox (Transformation|GetActorLocation) _movetarget) _movetarget) false false))
    (:then_1
      (for _array_element (Variables|Default|GetBoids)
        (bind _return (CallFunction|SetMaxForce _array_element))
        (bind _return_2 (CallFunction|SetMaxSpeed _return))
        (bind _return_3 (CallFunction|SetSepWeight _return_2))
        (bind _return_4 (CallFunction|SetAliWeight _return_3))
        (bind _return_5 (CallFunction|SetCohWeight _return_4))
        (bind _return_6 (CallFunction|SettoTargetWeight _return_5))
        (CallFunction|SetMaxTurnRate _return_6)))))

(fn ConstructionScript)

(fn SetBoidParameters
  (params (Boid :type Boid%20Object%20Reference) (MaxForce :type Float%20%28single-precision%29) (MaxSpeed :type Float%20%28single-precision%29) (SepWeight :type Float%20%28single-precision%29) (AliWeight :type Float%20%28single-precision%29) (CohWeight :type Float%20%28single-precision%29) (ToTargetWeight :type Float%20%28single-precision%29) (MaxTurnRate :type Float%20%28single-precision%29))
  (Variables|/Game/Flocking/Blueprint/Boid.Boid_C|SetMaxForce Boid MaxForce)
  (Variables|/Game/Flocking/Blueprint/Boid.Boid_C|SetMaxSpeed Boid MaxSpeed)
  (Variables|/Game/Flocking/Blueprint/Boid.Boid_C|SetSepWeight Boid SepWeight)
  (Variables|/Game/Flocking/Blueprint/Boid.Boid_C|SetAliWeight Boid AliWeight)
  (Variables|/Game/Flocking/Blueprint/Boid.Boid_C|SetCohWeight Boid CohWeight)
  (Variables|/Game/Flocking/Blueprint/Boid.Boid_C|SetToTargetWeight Boid ToTargetWeight)
  (Variables|/Game/Flocking/Blueprint/Boid.Boid_C|SetMaxTurnRate Boid MaxTurnRate))

(fn SetMaxForce
  (params (Boid :type Boid%20Object%20Reference))
  (Variables|/Game/Flocking/Blueprint/Boid.Boid_C|SetMaxForce Boid (Default|GetForceValue (Variables|Default|GetWID_Flocking)))
  (return Boid))

(fn SetMaxSpeed
  (params (Boid :type Boid%20Object%20Reference))
  (Variables|/Game/Flocking/Blueprint/Boid.Boid_C|SetMaxSpeed Boid (Default|GetSpeedValue (Variables|Default|GetWID_Flocking)))
  (return Boid))

(fn SetSepWeight
  (params (Boid :type Boid%20Object%20Reference))
  (Variables|/Game/Flocking/Blueprint/Boid.Boid_C|SetSepWeight Boid (Default|GetSepWeightValue (Variables|Default|GetWID_Flocking)))
  (return Boid))

(fn SetAliWeight
  (params (Boid :type Boid%20Object%20Reference))
  (Variables|/Game/Flocking/Blueprint/Boid.Boid_C|SetAliWeight Boid (Default|GetAliWeightValue (Variables|Default|GetWID_Flocking)))
  (return Boid))

(fn SetCohWeight
  (params (Boid :type Boid%20Object%20Reference))
  (Variables|/Game/Flocking/Blueprint/Boid.Boid_C|SetCohWeight Boid (Default|GetCohWeightValue (Variables|Default|GetWID_Flocking)))
  (return Boid))

(fn SettoTargetWeight
  (params (Boid :type Boid%20Object%20Reference))
  (Variables|/Game/Flocking/Blueprint/Boid.Boid_C|SetToTargetWeight Boid (Default|GettoTargetWeightValue (Variables|Default|GetWID_Flocking)))
  (return Boid))

(fn SetMaxTurnRate
  (params (Boid :type Boid%20Object%20Reference))
  (return Boid))